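; Player tank pawn Blueprint that enables firing at BeginPlay and feeds the tank's health and ammo to the HUD.
; Every Tick it casts the game mode to BP_TankGameModeBase and pushes the health ratio, current ammo and max ammo to that game mode's HPWidget.
; The HUD updates by per-frame polling, and the construction script is empty.
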(event EventTick
  (params (DeltaSeconds :type Float%20%28single-precision%29))
  (bind _health (Variables|Default|GetHealth))
  (bind _asbp_tank_game_mode_base (Utilities|Casting|CastToBP_TankGameModeBase (Game|GetGameMode)))
  (Default|ShowHP (Variables|/Game/BP/BP_TankGameModeBase.BP_TankGameModeBase_C|GetHPWidget _asbp_tank_game_mode_base) (/ (Variables|/Script/ToonTanks.HealthComponent|GetHealth _health) (Variables|/Script/ToonTanks.HealthComponent|GetMaxHealth _health)))
  (Default|ShowCurrentAmmo (Variables|/Game/BP/BP_TankGameModeBase.BP_TankGameModeBase_C|GetHPWidget _asbp_tank_game_mode_base) (Variables|Default|GetCurrentAmmo))
  (Default|ShowMaxAmmo (Variables|/Game/BP/BP_TankGameModeBase.BP_TankGameModeBase_C|GetHPWidget _asbp_tank_game_mode_base) (Variables|Default|GetMaxAmmo)))

(event EventBeginPlay
  (Variables|Default|SetbCanFire true))

(fn ConstructionScript)